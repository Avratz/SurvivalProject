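; Need Blueprint that models a single clamped value, such as a character need, that changes over time.
; TickValue applies a change-over-time rate scaled by the supplied delta, while Increase, Decrease and Set adjust or overwrite the current value directly.
; Every write clamps CurrentValue between zero and MaxValue, and a ClampAndSet function provides the same clamped assignment.
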(event `TickValue`
  (params (Delta :type "Float (double-precision)"))
  (set `self.CurrentValue` (`KismetMathLibrary.FClamp` (+ (* Delta (`self.ChangeOverTimeRate`)) (`self.CurrentValue`)) 0.0 (`self.MaxValue`))))

(event `Increase`
  (params (Amount :type "Float (double-precision)"))
  (set `self.CurrentValue` (`KismetMathLibrary.FClamp` (+ Amount (`self.CurrentValue`)) 0.0 (`self.MaxValue`))))

(event `Decrease`
  (params (Amount :type "Float (double-precision)"))
  (set `self.CurrentValue` (`KismetMathLibrary.FClamp` (- (`self.CurrentValue`) Amount) 0.0 (`self.MaxValue`))))

(event `Set`
  (params (NewValue :type "Float (double-precision)"))
  (set `self.CurrentValue` (`KismetMathLibrary.FClamp` NewValue 0.0 (`self.MaxValue`))))

(fn `ClampAndSet`
  (params (Value :type "Float (double-precision)"))
  (set `self.CurrentValue` (`KismetMathLibrary.FClamp` Value 0.0 (`self.MaxValue`))))